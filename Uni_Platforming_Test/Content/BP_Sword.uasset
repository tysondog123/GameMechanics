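; Thrown sword actor that flies toward a goal transform on behalf of a player and stops when it hits something.
; SwordFly stores the player, rotates the sword and plays a timeline that lerps from the current transform to the goal without sweeping.
; Any actor overlap sets HitWall, which stops the timeline on its next update.
; The timeline's Finished pin calls SwordReturn on the player.
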(event Custom|SwordFly
  (params (Player :type BP%20Platforming%20Character%20Object%20Reference) (Angle :type Rotator) (Goal :type Transform))
  (Variables|Default|SetPlayer Player)
  (Transformation|SetRelativeRotation (Variables|Default|GetSword) Angle false false)
  (bind _swordtrack_ (Timeline|Timeline Play)
    (:Update
      (Transformation|SetActorRelativeTransform (Math|Transform|Lerp(Transform) (Transformation|GetActorTransform) Goal _swordtrack_) false false)
      (if (Variables|Default|GetHitWall)
        (Timeline|Timeline Stop)))
    (:Finished
      (Default|SwordReturn (Variables|Default|GetPlayer)))))

(event EventBeginPlay)

(event EventTick
  (params (DeltaSeconds :type Float%20%28single-precision%29)))

(event Collision|EventActorBeginOverlap
  (params (OtherActor :type Actor%20Object%20Reference))
  (if true
    (Variables|Default|SetHitWall true)))

(fn ConstructionScript)