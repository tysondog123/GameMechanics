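; BP_PushCubeGoalBoss is a goal trigger for push cubes that exposes a weak point on a boss.
; When a BP_PushCube overlaps its Box and the boss has no weak point, it adds one to the boss and destroys the Box, so the goal fires only once.
; It plays an unlock sound and confetti particles, then after a short delay stops physics simulation on the cube.
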(event OnComponentBeginOverlap(Box)
  (params (OverlappedComponent :type Primitive%20Component%20Object%20Reference) (OtherActor :type Actor%20Object%20Reference) (OtherComp :type Primitive%20Component%20Object%20Reference) (OtherBodyIndex :type Integer) (bFromSweep :type Boolean) (SweepResult :type Hit%20Result%20Structure%20%28by%20ref%29))
  (bind _boss (Variables|Default|GetBoss))
  (bind _asbp_push_cube (Utilities|Casting|CastToBP_PushCube OtherActor))
  (if (not (Variables|/Game/BluePrints/BP_Boss.BP_Boss_C|GetHasWeakPoint _boss))
    (Default|AddWeakPoint _boss)
    (Components|DestroyComponent (Variables|Default|GetBox))
    (Audio|PlaySoundatLocation "/Game/Audio/SFX/Push_cube_unlock.Push_cube_unlock" (Transformation|GetActorLocation) "0, 0, 0" 1.0 1.0 0.0 0 0 0 0)
    (Niagara|ResetSystem (Variables|Default|GetPS_Confeti))
    (Utilities|FlowControl|Delay 1.0)
    (Physics|SetSimulatePhysics (Variables|/Game/BluePrints/BP_PushCube.BP_PushCube_C|GetCube _asbp_push_cube) false)))

(event EventBeginPlay)

(event Collision|EventActorBeginOverlap
  (params (OtherActor :type Actor%20Object%20Reference)))

(event EventTick
  (params (DeltaSeconds :type Float%20%28single-precision%29)))

(fn ConstructionScript)