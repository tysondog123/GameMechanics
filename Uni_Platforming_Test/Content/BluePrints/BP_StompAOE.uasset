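; BP_StompAOE is a short-lived stomp area attack that damages the player and knocks them away.
; On BeginPlay, a timeline grows the mesh horizontally, then destroys the actor when it finishes.
; The mesh's overlap with BP_PlayerCharacter applies damage once, guarded by a Hit flag.
; If the damage would not be lethal, it also launches the player upward and outward from the stomp's origin.
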(event OnComponentBeginOverlap(StaticMesh)
  (params (OverlappedComponent :type Primitive%20Component%20Object%20Reference) (OtherActor :type Actor%20Object%20Reference) (OtherComp :type Primitive%20Component%20Object%20Reference) (OtherBodyIndex :type Integer) (bFromSweep :type Boolean) (SweepResult :type Hit%20Result%20Structure%20%28by%20ref%29))
  (bind _returnvalue (Game|GetPlayerCharacter 0))
  (bind _returnvalue_2 (Game|GetPlayerCharacter 0))
  (bind _returnvalue_3 (Transformation|GetActorLocation))
  (bind _returnvalue_4 (Transformation|GetActorLocation _returnvalue_2))
  (bind _returnvalue_5 (- _returnvalue_4 _returnvalue_3))
  (bind _returnvalue_6 (Math|Vector|Normalize _returnvalue_5))
  (bind _returnvalue_7 (* _returnvalue_6 2e+03))
  (bind _asbp_player_character (Utilities|Casting|CastToBP_PlayerCharacter OtherActor))
  (if (not (Variables|Default|GetHit))
    (if (<= (- (Variables|/Game/BluePrints/BP_PlayerCharacter.BP_PlayerCharacter_C|GetHP _asbp_player_character) 5.0) 0.0)
      (Game|Damage|ApplyDamage _returnvalue 5.0 0 0)
      (Variables|Default|SetHit true)
      (else
        (Game|Damage|ApplyDamage _returnvalue 5.0 0 0)
        (Variables|Default|SetHit true)
        (Character|LaunchCharacter (Game|GetPlayerCharacter 0) (Math|Vector|MakeVector (.x _returnvalue_7) (.y _returnvalue_7) 2e+03) false false)))))

(event EventBeginPlay
  (bind _stomp_size (Timeline|Stomp_Grow PlayFromStart)
    (:Update
      (Transformation|SetRelativeScale3D (Variables|Default|GetStaticMesh) (Math|Vector|Lerp(Vector) "1.000000,1.000000,1.000000" "4.000000,4.000000,1.000000" _stomp_size)))
    (:Finished
      (Actor|DestroyActor))))

(event Collision|EventActorBeginOverlap
  (params (OtherActor :type Actor%20Object%20Reference)))

(event EventTick
  (params (DeltaSeconds :type Float%20%28single-precision%29)))

(fn ConstructionScript)