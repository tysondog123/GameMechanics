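; BP_Projectile is a projectile that flies toward the player and damages them on contact.
; After a short delay on BeginPlay, it locks a direction toward the player's current position, so it does not home.
; FlyForwads moves it by unswept world offsets, calling itself through a Delay instead of using Tick.
; Sphere1 overlap applies damage to a BP_PlayerCharacter and destroys the projectile on any overlapping actor.
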(event OnComponentBeginOverlap(Sphere1)
  (params (OverlappedComponent :type Primitive%20Component%20Object%20Reference) (OtherActor :type Actor%20Object%20Reference) (OtherComp :type Primitive%20Component%20Object%20Reference) (OtherBodyIndex :type Integer) (bFromSweep :type Boolean) (SweepResult :type Hit%20Result%20Structure%20%28by%20ref%29))
  (bind _asbp_player_character (Utilities|Casting|CastToBP_PlayerCharacter OtherActor)
    (:then
      (Game|Damage|ApplyDamage _asbp_player_character 1.0 0 0)
      (Actor|DestroyActor))
    (:CastFailed
      (Actor|DestroyActor))))

(event Custom|FlyForwads
  (params (Direction :type Vector))
  (Transformation|AddActorWorldOffset (* Direction 2e+01))
  (Utilities|FlowControl|Delay 0.01)
  (CallFunction|FlyForwads Direction))

(event EventBeginPlay
  (Utilities|FlowControl|Delay 0.2)
  (CallFunction|FlyForwads (Math|Vector|Normalize (- (.location (Transformation|GetActorTransform (Game|GetPlayerCharacter 0))) (.location (Transformation|GetActorTransform))))))

(event EventTick
  (params (DeltaSeconds :type Float%20%28single-precision%29)))

(fn ConstructionScript)