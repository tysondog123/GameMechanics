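; BP_PunchAOE is a short-lived area-of-effect punch shockwave that damages and knocks back the player.
; On BeginPlay a timeline scales its static mesh from small to large, then the actor destroys itself when finished.
; The mesh's overlap applies damage to BP_PlayerCharacter and launches it outward and upward, with a Hit flag limiting this to once per instance.
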(event OnComponentBeginOverlap(StaticMesh)
  (params (OverlappedComponent :type Primitive%20Component%20Object%20Reference) (OtherActor :type Actor%20Object%20Reference) (OtherComp :type Primitive%20Component%20Object%20Reference) (OtherBodyIndex :type Integer) (bFromSweep :type Boolean) (SweepResult :type Hit%20Result%20Structure%20%28by%20ref%29))
  (bind _asbp_player_character (Utilities|Casting|CastToBP_PlayerCharacter OtherActor))
  (if (not (Variables|Default|GetHit))
    (Game|Damage|ApplyDamage _asbp_player_character 5.0 0 0)
    (Variables|Default|SetHit true)
    (Character|LaunchCharacter _asbp_player_character (Math|Vector|MakeVector (.x (* (Math|Vector|Normalize (- (Transformation|GetActorLocation _asbp_player_character) (Transformation|GetActorLocation))) 2e+03)) (.y (* (Math|Vector|Normalize (- (Transformation|GetActorLocation _asbp_player_character) (Transformation|GetActorLocation))) 2e+03)) 2e+03) false false)))

(event EventBeginPlay
  (bind _punchsize (Timeline|Timeline Play)
    (:Update
      (Transformation|SetRelativeScale3D (Variables|Default|GetStaticMesh) (Math|Vector|Lerp(Vector) "2.000000,2.000000,2.000000" "15.000000,15.000000,15.000000" _punchsize)))
    (:Finished
      (Actor|DestroyActor))))

(event Collision|EventActorBeginOverlap
  (params (OtherActor :type Actor%20Object%20Reference)))

(event EventTick
  (params (DeltaSeconds :type Float%20%28single-precision%29)))

(fn ConstructionScript)