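; BP_PushCubeGoal is a goal zone for push-cube puzzles that drives a linked Switch.
; When a BP_PushCube enters its Box, it calls Key on the Switch, plays an unlock sound and restarts a confetti particle system.
; When the cube leaves, it calls Lock on the Switch and plays a lock sound.
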(event OnComponentBeginOverlap(Box)
  (params (OverlappedComponent :type Primitive%20Component%20Object%20Reference) (OtherActor :type Actor%20Object%20Reference) (OtherComp :type Primitive%20Component%20Object%20Reference) (OtherBodyIndex :type Integer) (bFromSweep :type Boolean) (SweepResult :type Hit%20Result%20Structure%20%28by%20ref%29))
  (Utilities|Casting|CastToBP_PushCube OtherActor)
  (Default|Key (Variables|Default|GetSwitch))
  (Audio|PlaySoundatLocation "/Game/Audio/SFX/Push_cube_unlock.Push_cube_unlock" (Transformation|GetActorLocation) "0, 0, 0" 1.0 1.0 0.0 0 0 0 0)
  (Niagara|ResetSystem (Variables|Default|GetPS_Confeti)))

(event OnComponentEndOverlap(Box)
  (params (OverlappedComponent :type Primitive%20Component%20Object%20Reference) (OtherActor :type Actor%20Object%20Reference) (OtherComp :type Primitive%20Component%20Object%20Reference) (OtherBodyIndex :type Integer))
  (Utilities|Casting|CastToBP_PushCube OtherActor)
  (Default|Lock (Variables|Default|GetSwitch))
  (Audio|PlaySoundatLocation "/Game/Audio/SFX/Push_Cube_Lock.Push_Cube_Lock" (Transformation|GetActorLocation) "0, 0, 0" 1.0 1.0 0.0 0 0 0 0))

(event EventBeginPlay)

(event Collision|EventActorBeginOverlap
  (params (OtherActor :type Actor%20Object%20Reference)))

(event EventTick
  (params (DeltaSeconds :type Float%20%28single-precision%29)))

(fn ConstructionScript)