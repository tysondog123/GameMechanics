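; BP_TutorialUIPopup is a trigger actor that shows a tutorial popup on screen while the player is inside its Box.
; When a BP_PlayerCharacter begins overlapping the Box, it creates a BP_Tutorial widget, passes it the actor's InputText and adds it to the viewport.
; When the player character stops overlapping, it removes the stored widget from its parent.
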(event OnComponentBeginOverlap(Box)
  (params (OverlappedComponent :type Primitive%20Component%20Object%20Reference) (OtherActor :type Actor%20Object%20Reference) (OtherComp :type Primitive%20Component%20Object%20Reference) (OtherBodyIndex :type Integer) (bFromSweep :type Boolean) (SweepResult :type Hit%20Result%20Structure%20%28by%20ref%29))
  (Utilities|Casting|CastToBP_PlayerCharacter OtherActor)
  (bind _returnvalue (UserInterface|CreateWidget "/Game/BluePrints/UI/BP_Tutorial.BP_Tutorial_C"))
  (bind _output_get (Variables|Default|SetUI%20Component _returnvalue))
  (bind _asbp_tutorial (Utilities|Casting|CastToBP_Tutorial _output_get))
  (Variables|/Game/BluePrints/UI/BP_Tutorial.BP_Tutorial_C|SetInput%20Text _asbp_tutorial (Variables|Default|GetInput%20Text))
  (UserInterface|Viewport|AddtoViewport (Variables|Default|GetUI%20Component) 0))

(event OnComponentEndOverlap(Box)
  (params (OverlappedComponent :type Primitive%20Component%20Object%20Reference) (OtherActor :type Actor%20Object%20Reference) (OtherComp :type Primitive%20Component%20Object%20Reference) (OtherBodyIndex :type Integer))
  (Utilities|Casting|CastToBP_PlayerCharacter OtherActor)
  (Widget|RemovefromParent (Variables|Default|GetUI%20Component)))

(event EventBeginPlay)

(event Collision|EventActorBeginOverlap
  (params (OtherActor :type Actor%20Object%20Reference)))

(event EventTick
  (params (DeltaSeconds :type Float%20%28single-precision%29)))

(fn ConstructionScript)