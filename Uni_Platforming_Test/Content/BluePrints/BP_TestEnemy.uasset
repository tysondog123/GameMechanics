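; BP_TestEnemy is a test enemy Blueprint with hit points and rough player-chasing logic.
; Attack decrements HP and destroys the actor at zero or below.
; MoveToPlayer re-calls itself every 0.2 seconds, setting the relative transform from the player direction times Speed, an absolute set rather than an offset.
; The chain that caches the player character and starts movement is disconnected, and BeginPlay is empty.
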(event Custom|MoveToPlayer
  (Transformation|SetActorRelativeTransform (Math|Conversions|ToTransform(Vector) (* (Math|Vector|Normalize (- (Transformation|GetActorLocation (Variables|Default|GetPlayer)) (Transformation|GetActorLocation))) (Variables|Default|GetSpeed))) false false)
  (Utilities|FlowControl|Delay 0.2)
  (CallFunction|MovetoPlayer))

(event EventBeginPlay)

(event Collision|EventActorBeginOverlap
  (params (OtherActor :type Actor%20Object%20Reference)))

(event EventTick
  (params (DeltaSeconds :type Float%20%28single-precision%29)))

(event EventAttack
  (bind _result (Math|Float|DecrementFloat (Variables|Default|GetHP))
    (:%20%20
      (bind _output_get (Variables|Default|SetHP _result))
      (if (<= _output_get 0.0)
        (Actor|DestroyActor)))))

(fn ConstructionScript)