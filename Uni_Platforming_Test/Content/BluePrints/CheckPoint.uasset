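; Checkpoint actor that updates the player's respawn point in the platforming game mode.
; When the player character overlaps its Box, it writes the box's location into the SpawnTransform of BP_PlatformingGameMode.
; It then swaps the mesh to a gold material, plays an unlock sound and resets the confetti particle system.
; The Box destroys itself afterwards, so each checkpoint triggers only once.
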(event OnComponentBeginOverlap(Box)
  (params (OverlappedComponent :type Primitive%20Component%20Object%20Reference) (OtherActor :type Actor%20Object%20Reference) (OtherComp :type Primitive%20Component%20Object%20Reference) (OtherBodyIndex :type Integer) (bFromSweep :type Boolean) (SweepResult :type Hit%20Result%20Structure%20%28by%20ref%29))
  (if (== OtherActor (Game|GetPlayerCharacter 0))
    (bind _asbp_platforming_game_mode (Utilities|Casting|CastToBP_PlatformingGameMode (Game|GetGameMode)))
    (Variables|/Game/Variant_Platforming/Blueprints/BP_PlatformingGameMode.BP_PlatformingGameMode_C|SetSpawn%20Transform _asbp_platforming_game_mode (Math|Conversions|ToTransform(Vector) (.location (Transformation|GetWorldTransform (Variables|Default|GetBox)))))
    (Rendering|Material|SetMaterial (Variables|Default|GetStaticMesh) 0 "/Game/StarterContent/Materials/M_Metal_Gold.M_Metal_Gold")
    (Audio|PlaySoundatLocation "/Game/Audio/SFX/Push_cube_unlock.Push_cube_unlock" (Transformation|GetActorLocation) "0, 0, 0" 1.0 1.0 0.0 0 0 0 0)
    (Components|DestroyComponent (Variables|Default|GetBox))
    (Niagara|ResetSystem (Variables|Default|GetPS_Confeti))))

(event EventBeginPlay)

(event Collision|EventActorBeginOverlap
  (params (OtherActor :type Actor%20Object%20Reference)))

(event EventTick
  (params (DeltaSeconds :type Float%20%28single-precision%29)))

(fn ConstructionScript)