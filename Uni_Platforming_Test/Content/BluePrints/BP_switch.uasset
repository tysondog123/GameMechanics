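; BP_switch is a one-use switch that counts toward opening its target door and can be locked.
; Lock and Key events raise and lower a lock counter, showing the cube or, at zero, hiding it with a glass-breaking sound.
; When unlocked, CallOpenDoor increments the door's pressed count, destroys the switch, and calls OpenDoor once the door's required count is reached.
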(event Custom|Key
  (bind _result (Math|Float|DecrementFloat (Variables|Default|GetLocked))
    (:%20%20
      (Variables|BP_switch_C|SetLocked self _result)
      (if (<= (Variables|Default|GetLocked) 0.0)
        (Development|SetHiddeninGame (Variables|Default|GetCube) true false)
        (Audio|PlaySoundatLocation "/Game/Audio/SFX/glass-breaking.glass-breaking" (Transformation|GetActorLocation) "0, 0, 0" 1.0 1.0 0.0 0 0 0 0)))))

(event Custom|Lock
  (bind _result (Math|Float|IncrementFloat (Variables|Default|GetLocked))
    (:%20%20
      (Variables|BP_switch_C|SetLocked self _result)
      (Development|SetHiddeninGame (Variables|Default|GetCube) false false))))

(event EventBeginPlay)

(event Collision|EventActorBeginOverlap
  (params (OtherActor :type Actor%20Object%20Reference)))

(event EventTick
  (params (DeltaSeconds :type Float%20%28single-precision%29)))

(event EventCallOpenDoor
  (bind _targetdoor (Variables|Default|GetTargetDoor))
  (if (<= (Variables|Default|GetLocked) 0.0)
    (if (not (Variables|Default|GetHas%20Been%20Pressed))
      (Variables|Default|SetHas%20Been%20Pressed true)
      (bind _result (Math|Integer|IncrementInt (Variables|/Game/BluePrints/BP_Door.BP_Door_C|GetSwitches%20presed _targetdoor))
        (:%20%20
          (bind _output_get (Variables|/Game/BluePrints/BP_Door.BP_Door_C|SetSwitches%20presed _targetdoor _result))
          (Actor|DestroyActor)
          (if (>= _output_get (Variables|/Game/BluePrints/BP_Door.BP_Door_C|GetNumberToOpen _targetdoor))
            (Default|OpenDoor _targetdoor)))))))

(fn ConstructionScript)