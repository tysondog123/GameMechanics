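; BP_Test_switch is a one-use test switch that helps open a linked TargetDoor.
; When CallOpenDoor fires for the first time, it marks itself pressed, increments the door's pressed-switch count and destroys itself.
; It then opens the door if that count has reached the door's NumberToOpen threshold, so several switches can share one door.
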(event EventBeginPlay)

(event Collision|EventActorBeginOverlap
  (params (OtherActor :type Actor%20Object%20Reference)))

(event EventTick
  (params (DeltaSeconds :type Float%20%28single-precision%29)))

(event EventCallOpenDoor
  (bind _targetdoor (Variables|Default|GetTargetDoor))
  (if (not (Variables|Default|GetHas%20Been%20Pressed))
    (Variables|Default|SetHas%20Been%20Pressed true)
    (bind _result (Math|Integer|IncrementInt (Variables|/Game/BluePrints/BP_Door.BP_Door_C|GetSwitches%20presed _targetdoor))
      (:%20%20
        (bind _output_get (Variables|/Game/BluePrints/BP_Door.BP_Door_C|SetSwitches%20presed _targetdoor _result))
        (Actor|DestroyActor)
        (if (>= _output_get (Variables|/Game/BluePrints/BP_Door.BP_Door_C|GetNumberToOpen _targetdoor))
          (Default|OpenDoor _targetdoor))))))

(fn ConstructionScript)